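; Game manager Blueprint that creates local players and spawns an Agua pawn for each at BeginPlay, after calling GetPlayerScreenWidgetGeometry.
; The construction script caches all PlayerStart actors.
; SpawnPlayer matches their tags to each player index, creates that player and spawns Agua at the start.
; Possession goes through the player character's LastHitBy controller reference, and each pawn is stored in the Player array.
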(event EventBeginPlay
  (Class|WidgetLayoutLibrary|GetPlayerScreenWidgetGeometry)
  (CallFunction|SpawnPlayer))

(fn ConstructionScript
  (bind _outactors (Actor|GetAllActorsOfClass "/Script/Engine.PlayerStart"))
  (Variables|Default|Setplayerstartarray _outactors))

(fn SpawnPlayer
  (for _index (range 0 (- (Variables|Default|Getmaxplayer%20acount) 1))
    (Variables|Default|Setindex _index)
    (for _array_element (Variables|Default|Getplayerstartarray)
      (if (Actor|ActorHasTag _array_element (Utilities|String|StringToName (Utilities|String|ToString(Integer) (Variables|Default|Getindex))))
        (Class|GameplayStatics|CreatePlayer (Variables|Default|Getindex))
        (bind _returnvalue (Game|SpawnActorfromClass "/Game/robot/agua.agua_C" (Transformation|GetActorTransform _array_element) "AlwaysSpawn" 0 0))
        (Pawn|Possess (Variables|/Script/Engine.Pawn|GetLastHitBy (Game|GetPlayerCharacter (Variables|Default|Getindex))) _returnvalue)
        (Utilities|Array|AddUnique (Variables|Default|Getplayer) _returnvalue)))))